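; BP_EQS_AmmoBoxContext is an EQS context that supplies a set of locations beside ammo boxes for AI environment queries.
; It gathers every BP_AmmoBox in the level and, for each, adds a point offset along the box's right vector and raised above it.
; The resulting location set is returned from ProvideLocationsSet, regardless of which querier runs the query.
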(fn ProvideLocationsSet
  (params (QuerierObject :type Object%20Object%20Reference) (QuerierActor :type Actor%20Object%20Reference))
  (bind _outactors (Actor|GetAllActorsOfClass "/Game/GameDevSG/Blueprints/Interactables/AmmoBox/BP_AmmoBox.BP_AmmoBox_C"))
  (for _array_element _outactors
    (Utilities|Array|Add (Variables|Default|GetResulting%20Location%20Set) (Math|Vector|MakeVector (.x (+ (Transformation|GetActorLocation _array_element) (* (Transformation|GetActorRightVector _array_element) 1.2e+02))) (.y (+ (Transformation|GetActorLocation _array_element) (* (Transformation|GetActorRightVector _array_element) 1.2e+02))) (+ (.z (+ (Transformation|GetActorLocation _array_element) (* (Transformation|GetActorRightVector _array_element) 1.2e+02))) 1e+02))))
  (return (Variables|Default|GetResulting%20Location%20Set)))