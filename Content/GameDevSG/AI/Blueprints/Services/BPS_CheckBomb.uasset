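; Behavior tree service for the Rush mode AI that picks a bomb for the pawn to interact with when the search starts.
; It shuffles the game state's bomb list, skips two bomb states, and matches each bomb's state against whether it shares the pawn's team.
; It writes the result to a blackboard bool, stopping at the first match to store a location offset along world X from that bomb.
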(event EventReceiveSearchStartAI
  (params (OwnerController :type AI%20Controller%20Object%20Reference) (ControlledPawn :type Pawn%20Object%20Reference))
  (bind _asbp_rush_gs (Utilities|Casting|CastToBP_Rush_GS (Game|GetGameState)))
  (Utilities|Array|Shuffle (Variables|/Game/FPS/Blueprints/GameModes/Rush/BP_Rush_GS.BP_Rush_GS_C|GetBombRef _asbp_rush_gs))
  (bind _array_element (Utilities|Array|ForEachLoopwithBreak (Variables|/Game/FPS/Blueprints/GameModes/Rush/BP_Rush_GS.BP_Rush_GS_C|GetBombRef _asbp_rush_gs) :!label _label)
    (:LoopBody
      (Utilities|IsValid _array_element
        (:Is%20Valid
          (if (and (Utilities|Enum|NotEqual(Enum) (Variables|/Game/FPS/Blueprints/GameObjectives/RushObjective/BP_RushObjective.BP_RushObjective_C|GetBombState _array_element) "NewEnumerator3") (Utilities|Enum|NotEqual(Enum) (Variables|/Game/FPS/Blueprints/GameObjectives/RushObjective/BP_RushObjective.BP_RushObjective_C|GetBombState _array_element) "NewEnumerator2"))
            (Class|BTFunctionLibrary|SetBlackboardValueasBool (Variables|Default|GetInteractBombKey) (not (Class|KismetMathLibrary|XORBoolean (Utilities|Enum|Equal(Enum) (Variables|/Game/FPS/Blueprints/GameObjectives/RushObjective/BP_RushObjective.BP_RushObjective_C|GetBombState _array_element) "NewEnumerator1") (== (Variables|/Game/FPS/Blueprints/GameObjectives/RushObjective/BP_RushObjective.BP_RushObjective_C|GetTeam _array_element) (Default|GetTeam (Actor|GetComponentbyClass (Variables|/Script/Engine.Pawn|GetPlayerState ControlledPawn) "/Game/GameDevSG/Blueprints/BlueprintsComponents/AC_Team.AC_Team_C"))))))
            (if (not (Class|KismetMathLibrary|XORBoolean (Utilities|Enum|Equal(Enum) (Variables|/Game/FPS/Blueprints/GameObjectives/RushObjective/BP_RushObjective.BP_RushObjective_C|GetBombState _array_element) "NewEnumerator1") (== (Variables|/Game/FPS/Blueprints/GameObjectives/RushObjective/BP_RushObjective.BP_RushObjective_C|GetTeam _array_element) (Default|GetTeam (Actor|GetComponentbyClass (Variables|/Script/Engine.Pawn|GetPlayerState ControlledPawn) "/Game/GameDevSG/Blueprints/BlueprintsComponents/AC_Team.AC_Team_C")))))
              (AI|BehaviorTree|SetBlackboardValueasVector (Variables|Default|GetLocationKey) (Math|Vector|MakeVector (+ (.x (Transformation|GetActorLocation _array_element)) 1e+02) (.y (Transformation|GetActorLocation _array_element)) (.z (Transformation|GetActorLocation _array_element))))
              (goto _label Break))))))))