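; Behavior tree task that has an AI pawn interact with nearby Search and Destroy objectives.
; If the pawn is alive, it loops over the game state's objectives and calls the AI bomb interaction on Search and Destroy ones within a fixed radius.
; It then clears the interact-bomb blackboard key and finishes successfully.
; A dead pawn skips all of this, including the finish call.
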(event EventReceiveExecuteAI
  (params (OwnerController :type AI%20Controller%20Object%20Reference) (ControlledPawn :type Pawn%20Object%20Reference))
  ;[1 1 1] Interact with objective
  (if (not (Default|IsDead (Actor|GetComponentbyClass ControlledPawn "/Game/GameDevSG/Blueprints/BlueprintsComponents/AC_Health.AC_Health_C")))
    (bind _asbp_base_gs (Utilities|Casting|CastToBP_Base_GS (Game|GetGameState)))
    (for _array_element (Variables|/Game/FPS/Blueprints/GameModes/BP_Base_GS.BP_Base_GS_C|GetObjectives _asbp_base_gs)
      (Utilities|IsValid _array_element
        (:Is%20Valid
          (if (<= (Math|Vector|VectorLength (- (Transformation|GetActorLocation _array_element) (Transformation|GetActorLocation ControlledPawn))) 5e+02)
            (bind _asbp_search_and_destroy_objective (Utilities|Casting|CastToBP_SearchAndDestroyObjective _array_element))
            (Default|AIBombInteract _asbp_search_and_destroy_objective ControlledPawn)))))
    (Class|BTFunctionLibrary|SetBlackboardValueasBool (Variables|Default|GetInteractBombKey) false)
    (AI|BehaviorTree|FinishExecute true)))