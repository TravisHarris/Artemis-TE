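; Player controller component that provides in-game text chat with all-player and team-only channels.
; BeginPlay creates the WB_Chat widget for the local player, and two input actions open its entry box in either mode.
; Server_GetChatMessage loops over the GameState's PlayerArray, filters by AC_Team for team chat, and forwards sender and text to each recipient's chat component.
; Client_UpdateChat and SendServerMessage write player and server messages into the chat window.
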(event Custom|SendServerMessage
  (params (Message :type Text))
  (bind _wb_chatwindow (Variables|Default|GetWB_ChatWindow))
  ;[0 0 0] Server Send message
  (Utilities|IsValid _wb_chatwindow
    (:Is%20Valid
      (Default|ServerMessage (Variables|/Game/GameDevSG/UI/Chat/WB_Chat.WB_Chat_C|GetChatWindow _wb_chatwindow) "" Message false))))

(event Custom|OpenChat
  (params (bTeamChat :type Boolean))
  (bind _wb_chatwindow (Variables|Default|GetWB_ChatWindow))
  (bind _chatwindow (Variables|/Game/GameDevSG/UI/Chat/WB_Chat.WB_Chat_C|GetChatWindow _wb_chatwindow))
  ;[0 0 0] Open Chat
  (Default|InitChatEntry _chatwindow bTeamChat)
  (Class|PlayerController|SetMouseCursorWidget (Game|GetPlayerController 0) "None" _chatwindow)
  (Widget|SetKeyboardFocus (Variables|/Game/GameDevSG/UI/Chat/WB_ChatWindow.WB_ChatWindow_C|GetChatEntry _chatwindow))
  (Class|UserWidget|StopAllAnimations _chatwindow))

(event Custom|Client_UpdateChat
  (params (Sender :type Text) (text :type Text) (bTeamChat :type Boolean))
  (bind _wb_chatwindow (Variables|Default|GetWB_ChatWindow))
  ;[0 0 0] Update Chat
  (Utilities|IsValid _wb_chatwindow
    (:Is%20Valid
      (Default|UpdateChatWindow (Variables|/Game/GameDevSG/UI/Chat/WB_Chat.WB_Chat_C|GetChatWindow _wb_chatwindow) Sender text bTeamChat))))

(event Custom|Server_GetChatMessage
  (params (TextToSend :type Text) (bTeamChat :type Boolean) (SenderPC :type Player%20Controller%20Object%20Reference))
  ;[0 0 0] Server get chat message
  (Variables|Default|SetSenderText TextToSend)
  (Variables|Default|SetSenderName (Utilities|Text|ToText(String) (PlayerState|GetPlayerName (Variables|/Script/Engine.Controller|GetPlayerState SenderPC))))
  (for _array_element (Variables|/Script/Engine.GameStateBase|GetPlayerArray (Game|GetGameState))
    (Utilities|IsValid (Game|GetPlayerController _array_element)
      (:Is%20Valid
        (if bTeamChat
          (if (== (Default|GetTeam (Actor|GetComponentbyClass _array_element "/Game/GameDevSG/Blueprints/BlueprintsComponents/AC_Team.AC_Team_C")) (Default|GetTeam (Actor|GetComponentbyClass (Variables|/Script/Engine.Controller|GetPlayerState SenderPC) "/Game/GameDevSG/Blueprints/BlueprintsComponents/AC_Team.AC_Team_C")))
            (CallFunction|ClientUpdateChat (Actor|GetComponentbyClass (Game|GetPlayerController _array_element) "AC_ChatSystem_C") (Variables|Default|GetSenderName) (Variables|Default|GetSenderText) bTeamChat :!label _label)
            (Networking|ForceNetUpdate (Components|GetOwner)))
          (else
            (goto _label)))))))

(event Input|EnhancedActionEvents|EnhancedInputActionIA_OpenChat
  (params (ActionValue :type Boolean) (ElapsedSeconds :type Float%20%28double-precision%29) (TriggeredSeconds :type Float%20%28double-precision%29) (InputAction :type Input%20Action%20Object%20Reference :default "/Game/FPS/Inputs/InputActions/IA_OpenChat.IA_OpenChat"))
  ;[0 0 0] Input
  (CallFunction|OpenChat false))

(event Input|EnhancedActionEvents|EnhancedInputActionIA_OpenTeamChat
  (params (ActionValue :type Boolean) (ElapsedSeconds :type Float%20%28double-precision%29) (TriggeredSeconds :type Float%20%28double-precision%29) (InputAction :type Input%20Action%20Object%20Reference :default "/Game/FPS/Inputs/InputActions/IA_OpenTeamChat.IA_OpenTeamChat"))
  ;[0 0 0] Input
  (CallFunction|OpenChat true))

(event EventBeginPlay
  (bind _returnvalue (Game|GetPlayerController 0))
  ;[0 0 0] Begin Play
  (if (Pawn|IsLocalController _returnvalue)
    (bind _returnvalue_2 (UserInterface|CreateWidget "/Game/GameDevSG/UI/Chat/WB_Chat.WB_Chat_C" _returnvalue))
    (bind _output_get (Variables|Default|SetWB_ChatWindow _returnvalue_2))
    (UserInterface|Viewport|AddtoViewport _output_get 2)))