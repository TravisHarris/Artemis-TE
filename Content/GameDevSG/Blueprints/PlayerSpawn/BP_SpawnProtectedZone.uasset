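; Spawn-protection zone actor that stops the local player from lingering in a spawn area belonging to another team.
; Box overlaps compare the player's AC_Team team, read from PlayerState, against SpawnTeam.
; An intruder gets a WB_ProtectedZoneWarning widget fed by a countdown timer, and both are cleared on exit.
; When the timer expires, self-instigated massive damage hits the player; construction sizes the box from BoxX and BoxY.
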(event OnComponentBeginOverlap(Box)
  (params (OverlappedComponent :type Primitive%20Component%20Object%20Reference) (OtherActor :type Actor%20Object%20Reference) (OtherComp :type Primitive%20Component%20Object%20Reference) (OtherBodyIndex :type Integer) (bFromSweep :type Boolean) (SweepResult :type Hit%20Result%20Structure%20%28by%20ref%29))
  ;[0 0 0] Overlap Events
  (if (== OtherActor (Game|Player|GetPlayerPawn 0))
    (Utilities|Casting|CastToCharacter OtherActor)
    (if (not (== (Default|GetTeam (Actor|GetComponentbyClass (Variables|/Script/Engine.Controller|GetPlayerState (Game|GetInstigatorController OtherActor)) "/Game/GameDevSG/Blueprints/BlueprintsComponents/AC_Team.AC_Team_C")) (Variables|Default|GetSpawnTeam)))
      (CallFunction|Warn true))))

(event OnComponentEndOverlap(Box)
  (params (OverlappedComponent :type Primitive%20Component%20Object%20Reference) (OtherActor :type Actor%20Object%20Reference) (OtherComp :type Primitive%20Component%20Object%20Reference) (OtherBodyIndex :type Integer))
  (bind _returnvalue (Game|GetInstigatorController OtherActor))
  ;[0 0 0] Overlap Events
  (if (== OtherActor (Game|Player|GetPlayerPawn 0))
    (Utilities|IsValid _returnvalue
      (:Is%20Valid
        (if (not (== (Default|GetTeam (Actor|GetComponentbyClass (Variables|/Script/Engine.Controller|GetPlayerState _returnvalue) "/Game/GameDevSG/Blueprints/BlueprintsComponents/AC_Team.AC_Team_C")) (Variables|Default|GetSpawnTeam)))
          (CallFunction|Warn false))))))

(event Custom|Warn
  (params (bShowWarning :type Boolean))
  ;[0 0 0] Overlap Events
  (if bShowWarning
    (bind _returnvalue (Utilities|Time|SetTimerbyEvent (delegate Custom|KillPlayerIntruder) (Variables|Default|GetTimeToLeave)))
    (bind _output_get (Variables|Default|SetLeaveProtectedZoneHandle _returnvalue))
    (bind _returnvalue_2 (UserInterface|CreateWidget "/Game/GameDevSG/UI/Gameplay/WB_ProtectedZoneWarning.WB_ProtectedZoneWarning_C" (Game|GetPlayerController 0) _output_get))
    (Utilities|IsValid _returnvalue_2
      (:Is%20Valid
        (bind _output_get_2 (Variables|Default|SetProtectedZoneWidget _returnvalue_2))
        (UserInterface|Viewport|AddtoViewport _output_get_2 0)))
    (else
      (Utilities|Time|ClearandInvalidateTimerbyHandle (Variables|Default|GetLeaveProtectedZoneHandle))
      (Utilities|IsValid (Variables|Default|GetProtectedZoneWidget)
        (:Is%20Valid
          (Widget|RemovefromParent (Variables|Default|GetProtectedZoneWidget)))))))

(event Custom|KillPlayerIntruder
  (bind _returnvalue (Game|Player|GetPlayerPawn 0))
  ;[0 0 0] Overlap Events
  (Game|Damage|ApplyDamage _returnvalue 1e+04 (Pawn|GetController _returnvalue) _returnvalue))

(fn ConstructionScript
  (Components|Box|SetBoxExtent (Variables|Default|GetBox) (Math|Vector|MakeVector (Variables|Default|GetBox_X) (Variables|Default|GetBox_Y) 3e+02) true))