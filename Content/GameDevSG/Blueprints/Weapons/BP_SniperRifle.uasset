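; BP_SniperRifle is a weapon Blueprint for a sniper rifle with a scope overlay.
; Aiming zeroes AimOffset, adds the scope widget and hides the first or third person mesh according to the controller's TPP setting; releasing restores these and stops camera shakes.
; Shots play FireShake while aiming and CS_FireWeapon otherwise.
; WeaponVisibility toggles owner visibility of the first person weapon mesh.
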(event EventPlayShotShake
  (bind _returnvalue (Game|GetPlayerCameraManager 0))
  (bind _returnvalue_2 (Game|Player|GetPlayerPawn 0))
  (bind _returnvalue_3 (Actor|GetComponentbyClass _returnvalue_2 "/Game/GameDevSG/Blueprints/BlueprintsComponents/AC_PawnInfo.AC_PawnInfo_C"))
  ;[0 0 0] FireShake
  (Utilities|IsValid _returnvalue_3
    (:Is%20Valid
      (Utilities|IsValid _returnvalue
        (:Is%20Valid
          (CameraShakes|StartCameraShake _returnvalue (select (Default|GetAiming _returnvalue_3) (Variables|Default|GetFireShake) "/Game/GameDevSG/Blueprints/CameraShake/CS_FireWeapon.CS_FireWeapon_C") 1.0 "CameraLocal" "0, 0, 0"))))))

(event EventOnBeginAiming
  (bind _returnvalue (Game|Player|GetPlayerPawn 0))
  ;[0 0 0] On Begin Amining
  (Variables|Default|SetAimOffset 0.0)
  (bind _returnvalue_2 (UserInterface|CreateWidget "/Game/GameDevSG/UI/Gameplay/WB_SniperScope.WB_SniperScope_C" (Game|GetPlayerController 0)))
  (bind _output_get (Variables|Default|SetSniperScopeRef _returnvalue_2))
  (UserInterface|Viewport|AddtoViewport _output_get -1)
  (if (Default|GetUseTPP (Actor|GetComponentbyClass (Game|GetPlayerController 0) "/Game/GameDevSG/Blueprints/BlueprintsComponents/AC_ControllerSettings.AC_ControllerSettings_C"))
    (Class|IPawnActions|HideTPPMesh(Message) _returnvalue)
    (else
      (Class|IPawnActions|HideFPPMesh(Message) _returnvalue))))

(event EventOnStopAiming
  (bind _returnvalue (Game|Player|GetPlayerPawn 0))
  (bind _returnvalue_2 (Game|GetPlayerController 0))
  (bind _returnvalue_3 (Actor|GetComponentbyClass _returnvalue_2 "/Game/GameDevSG/Blueprints/BlueprintsComponents/AC_ControllerSettings.AC_ControllerSettings_C"))
  ;[0 0 0] On End Aiming
  (Variables|Default|SetAimOffset 0.13)
  (Utilities|IsValid _returnvalue_2
    (:Is%20Valid
      (CameraShake|StopAllCameraShakes (Game|GetPlayerCameraManager 0) true)
      (bind _sniperscoperef (Variables|Default|GetSniperScopeRef)
        (:then
          (Widget|RemovefromParent _sniperscoperef))
        (:else
          _))
      (Utilities|IsValid _returnvalue_3
        (:Is%20Valid
          (if (Default|GetUseTPP _returnvalue_3)
            (Class|IPawnActions|ShowTPPMesh(Message) _returnvalue)
            (else
              (Class|IPawnActions|ShowFPPMesh(Message) _returnvalue))))))))

(fn ConstructionScript
  (|CallParentFunction))

(fn WeaponVisibility
  (params (bVisible :type Boolean))
  (Class|PrimitiveComponent|SetOwnerNoSee (Variables|Default|GetMeshFPP) (not bVisible)))